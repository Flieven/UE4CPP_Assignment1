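; Weapon Blueprint, by its name for projectile weapons, that fires from a single projectile barrel when primary fire is triggered.
; An active PrimaryFire event stores the controller and calls Fire with the ProjectileBarrel.
; The result of Fire feeds the Recoil component's DoRecoil as barrel recoils, along with the controller.
; The default BeginPlay, overlap and Tick events are disabled, and the construction script only calls its parent.
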(event EventBeginPlay
  (|CallParentFunction) ; This node is disabled and will not be called.\nDrag off pins to build functionality.
)

(event Collision|EventActorBeginOverlap
  (params (OtherActor :type Actor%20Object%20Reference))
  (|CallParentFunction OtherActor) ; This node is disabled and will not be called.\nDrag off pins to build functionality.
)

(event EventTick
  (params (DeltaSeconds :type Float%20%28single-precision%29))
  (|CallParentFunction DeltaSeconds) ; This node is disabled and will not be called.\nDrag off pins to build functionality.
)

(event EventPrimaryFire
  (params (controller :type Controller%20Object%20Reference) (active :type Boolean))
  (if active
    (bind _output_get (Variables|Default|SetController controller))
    (bind _returnvalue (Class|Weapon|Fire (Utilities|Array|MakeArray (Variables|Default|GetProjectileBarrel)) _output_get))
    (Class|RecoilComponent|DoRecoil (Variables|Default|GetRecoil) (Variables|Default|GetController) _returnvalue)))

(fn ConstructionScript
  (|CallParentFunction))