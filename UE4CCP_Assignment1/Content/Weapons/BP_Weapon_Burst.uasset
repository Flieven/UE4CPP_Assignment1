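; Burst-fire weapon Blueprint that fires a three-shot burst each time primary fire is activated.
; A sequence starts three staggered, evenly spaced delays into one shared fire step, so even the first shot is delayed and releasing fire does not cancel the burst.
; Each shot fires through the line trace barrel and passes its result to the Recoil component.
; An external reload event reloads that same barrel.
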(event EventBeginPlay
  (|CallParentFunction) ; This node is disabled and will not be called.\nDrag off pins to build functionality.
)

(event Collision|EventActorBeginOverlap
  (params (OtherActor :type Actor%20Object%20Reference))
  (|CallParentFunction OtherActor) ; This node is disabled and will not be called.\nDrag off pins to build functionality.
)

(event EventTick
  (params (DeltaSeconds :type Float%20%28single-precision%29))
  (|CallParentFunction DeltaSeconds) ; This node is disabled and will not be called.\nDrag off pins to build functionality.
)

(event EventPrimaryFire
  (params (controller :type Controller%20Object%20Reference) (active :type Boolean))
  (if active
    (Variables|Default|SetController controller)
    (Utilities|FlowControl|Sequence
      (:then_0
        (Utilities|FlowControl|Delay 0.2))
      (:then_1
        (Utilities|FlowControl|Delay 0.4))
      (:then_2
        (Utilities|FlowControl|Delay 0.6)))
    (bind _returnvalue (Class|Weapon|Fire (Utilities|Array|MakeArray (Variables|Default|GetLinetraceBarrel)) (Variables|Default|GetController)))
    (Class|RecoilComponent|DoRecoil (Variables|Default|GetRecoil) (Variables|Default|GetController) _returnvalue)))

(event EventReloadExtrenally
  (params (Caller :type Actor%20Object%20Reference))
  (Class|Weapon|Reload Caller (Variables|Default|GetLinetraceBarrel)))

(fn ConstructionScript
  (|CallParentFunction))