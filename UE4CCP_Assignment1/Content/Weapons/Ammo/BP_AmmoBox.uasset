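; BP_AmmoBox is an ammo box actor that hovers and spins in place, apparently intended as a pickup.
; A Hover timeline started on BeginPlay adds its curve value to the current Z and a fixed yaw step on each update, so motion accumulates per frame.
; The sphere overlap event meant to add ammo is empty, and the ammo capacity and current-ammo functions are stubs returning zero.
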(event OnComponentBeginOverlap(SphereCollider)
  (params (OverlappedComponent :type Primitive%20Component%20Object%20Reference) (OtherActor :type Actor%20Object%20Reference) (OtherComp :type Primitive%20Component%20Object%20Reference) (OtherBodyIndex :type Integer) (bFromSweep :type Boolean) (SweepResult :type Hit%20Result%20Structure%20%28by%20ref%29))
  ;[1 0 0] Add Ammo
)

(event EventBeginPlay
  (bind _returnvalue (Transformation|GetActorLocation))
  (bind _returnvalue_2 (Transformation|GetActorRotation))
  ;[1 1 1] Idle Hovering & Rotating
  (bind _hovering (Timeline|Hover PlayFromStart)
    (:Update
      (Transformation|SetActorLocation (Math|Vector|MakeVector (.x _returnvalue) (.y _returnvalue) (+ (.z _returnvalue) _hovering)) false false)
      (Transformation|SetActorRotation (Math|Rotator|MakeRotator (.roll _returnvalue_2) (.pitch _returnvalue_2) (+ (.yaw _returnvalue_2) 0.2))))))

(fn ConstructionScript)

(fn GetAmmoCapacity
  (return 0))

(fn GetCurrentAmmo
  (return 0))