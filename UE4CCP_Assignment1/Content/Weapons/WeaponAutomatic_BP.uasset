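; Automatic weapon Blueprint that fires repeatedly while primary fire is active.
; PrimaryFire stores the controller and starts a looping timer, clearing it when input is released.
; Each timer tick fires the linetrace barrel and passes the resulting barrel recoils to the Recoil component.
; External reload requests forward the caller and barrel to Reload.
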(event Custom|CallFire
  (bind _returnvalue (Class|Weapon|Fire (Utilities|Array|MakeArray (Variables|Default|GetLinetraceBarrel)) (Variables|Default|GetController)))
  (Class|RecoilComponent|DoRecoil (Variables|Default|GetRecoil) (Variables|Default|GetController) _returnvalue))

(event EventBeginPlay
  (|CallParentFunction) ; This node is disabled and will not be called.\nDrag off pins to build functionality.
)

(event Collision|EventActorBeginOverlap
  (params (OtherActor :type Actor%20Object%20Reference))
  (|CallParentFunction OtherActor) ; This node is disabled and will not be called.\nDrag off pins to build functionality.
)

(event EventTick
  (params (DeltaSeconds :type Float%20%28single-precision%29))
  (|CallParentFunction DeltaSeconds) ; This node is disabled and will not be called.\nDrag off pins to build functionality.
)

(event EventPrimaryFire
  (params (controller :type Controller%20Object%20Reference) (active :type Boolean))
  (if active
    (Variables|Default|SetController controller)
    (bind _returnvalue (Utilities|Time|SetTimerbyEvent (delegate Custom|CallFire) 0.2 true))
    (Variables|Default|SetTimerHandle _returnvalue)
    (else
      (Utilities|Time|ClearandInvalidateTimerbyHandle (Variables|Default|GetTimerHandle)))))

(event EventReloadExtrenally
  (params (Caller :type Actor%20Object%20Reference))
  (Class|Weapon|Reload Caller (Variables|Default|GetLinetraceBarrel)))

(fn ConstructionScript
  (|CallParentFunction))